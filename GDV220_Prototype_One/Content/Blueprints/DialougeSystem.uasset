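; Dialogue actor that shows lines from an array in a HUD widget, advancing one line per Enter press.
; StartDialogue reveals the widget, shows the next line and blocks player movement; running out of lines hides it and restores movement.
; Looping dialogue resets its index at the end, though IsActive is never cleared.
; The sphere overlap event is empty, leaving the character cast and StartDialogue call disconnected.
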(event OnComponentBeginOverlap(Sphere)
  (params (OverlappedComponent :type Primitive%20Component%20Object%20Reference) (OtherActor :type Actor%20Object%20Reference) (OtherComp :type Primitive%20Component%20Object%20Reference) (OtherBodyIndex :type Integer) (bFromSweep :type Boolean) (SweepResult :type Hit%20Result%20Structure%20%28by%20ref%29)))

(event Custom|OnDialogueProceed
  (Development|PrintText "EnterPressed")
  (if (Variables|Default|GetisActive)
    (if (< (Variables|Default|GetPositionInArray) (Utilities|Array|Length (Variables|Default|GetDialougeArray)))
      (Default|UpdateText (Variables|Default|GetUI) (Utilities|Array|Get(acopy) (Variables|Default|GetDialougeArray) (Variables|Default|GetPositionInArray)))
      (Math|Integer|IncrementInt (Variables|Default|GetPositionInArray))
      (else
        (Widget|SetVisibility (Variables|Default|GetUI) "Hidden")
        (Input|SetIgnoreMoveInput (Game|GetPlayerController 0) false)
        (if (Variables|Default|GetisLooping)
          (Variables|Default|SetPositionInArray 0))))))

(event EventBeginPlay
  (bind _returnvalue (UserInterface|CreateWidget "/Game/Blueprints/HUD_Dialouge.HUD_Dialouge_C"))
  (bind _output_get (Variables|Default|SetUI _returnvalue))
  (UserInterface|Viewport|AddtoViewport _output_get 0)
  (Widget|SetVisibility _output_get "Hidden"))

(event Input|KeyboardEvents|Enter
  (params (Key :type Key%20Structure :default "None"))
  (:Pressed
    (CallFunction|OnDialogueProceed)))

(fn ConstructionScript)

(fn StartDialogue
  (Development|PrintString "Start Dialouge Called")
  (if (< (Variables|Default|GetPositionInArray) (Utilities|Array|Length (Variables|Default|GetDialougeArray)))
    (Default|UpdateText (Variables|Default|GetUI) (Utilities|Array|Get(acopy) (Variables|Default|GetDialougeArray) (Variables|Default|GetPositionInArray)))
    (Math|Integer|IncrementInt (Variables|Default|GetPositionInArray)
      (:%20%20
        (Widget|SetVisibility (Variables|Default|GetUI) "Visible")
        (Variables|Default|SetisActive true)
        (Input|SetIgnoreMoveInput (Game|GetPlayerController 0) true)))))