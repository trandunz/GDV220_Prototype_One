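; End-game trigger actor that swings a two-leaf gate open and starts the end-game fade HUD.
; The first box overlap sets a one-shot flag and plays a timeline rotating both gate meshes in opposite directions, lerping from their current world rotation into relative rotation.
; The fade widget appears only if that overlapping actor is the ThirdPersonCharacter; any actor opens the gate and consumes the trigger.
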(event OnComponentBeginOverlap(Box)
  (params (OverlappedComponent :type Primitive%20Component%20Object%20Reference) (OtherActor :type Actor%20Object%20Reference) (OtherComp :type Primitive%20Component%20Object%20Reference) (OtherBodyIndex :type Integer) (bFromSweep :type Boolean) (SweepResult :type Hit%20Result%20Structure%20%28by%20ref%29))
  (bind _sm_gate_r (Variables|Default|GetSM_Gate_R))
  (bind _sm_gate_l (Variables|Default|GetSM_Gate_L))
  (if (not (Variables|Default|GetIsGateOpen))
    (Utilities|FlowControl|Sequence
      (:then_0
        (Utilities|Casting|CastToThirdPersonCharacter OtherActor)
        (bind _returnvalue (UserInterface|CreateWidget "/Game/Blueprints/HUD_EndGameFade.HUD_EndGameFade_C"))
        (UserInterface|Viewport|AddtoViewport _returnvalue 0)
        (Variables|/Game/Blueprints/HUD_EndGameFade.HUD_EndGameFade_C|SetIsFading _returnvalue true))
      (:then_1
        (Variables|Default|SetIsGateOpen true))
      (:then_3
        (bind _gate_rotation (Timeline|GateOpening PlayFromStart)
          (:Update
            (Utilities|FlowControl|Sequence
              (:then_0
                (Transformation|SetRelativeRotation _sm_gate_r (Math|Rotator|Lerp(Rotator) (Transformation|GetWorldRotation _sm_gate_r) "0.000000,90.000000,0.000000" _gate_rotation) false false))
              (:then_1
                (Transformation|SetRelativeRotation _sm_gate_l (Math|Rotator|Lerp(Rotator) (Transformation|GetWorldRotation _sm_gate_l) "0,-90.000000, 0" _gate_rotation) false false)))))))))

(event EventBeginPlay)

(event Collision|EventActorBeginOverlap
  (params (OtherActor :type Actor%20Object%20Reference)))

(event EventTick
  (params (DeltaSeconds :type Float%20%28single-precision%29)))

(fn ConstructionScript)