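; Gate Blueprint that swings a two-leaf gate open when its Open event is called.
; A timeline's GateRotation track drives rotator lerps that turn the right and left meshes 90 degrees in opposite directions.
; Each update lerps from the current relative rotation rather than a stored start, so motion compounds along the curve.
; GateOpen is set only when the timeline finishes, blocking later calls, and no close logic exists.
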(event Custom|Open
  (bind _sm_gate_r (Variables|Default|GetSM_Gate_R))
  (bind _sm_gate_l (Variables|Default|GetSM_Gate_L))
  (if (not (Variables|Default|GetGateOpen))
    (bind _gate_rotation (Timeline|Timeline_0 PlayFromStart)
      (:Update
        (Utilities|FlowControl|Sequence
          (:then_0
            (Transformation|SetRelativeRotation _sm_gate_r (Math|Rotator|Lerp(Rotator) (Variables|/Script/Engine.SceneComponent|GetRelativeRotation _sm_gate_r) "0.000000,90.000000,0.000000" _gate_rotation) false false))
          (:then_1
            (Transformation|SetRelativeRotation _sm_gate_l (Math|Rotator|Lerp(Rotator) (Variables|/Script/Engine.SceneComponent|GetRelativeRotation _sm_gate_l) "0,-90.000000, 0" _gate_rotation) false false))))
      (:Finished
        (Variables|Default|SetGateOpen true)))))

(fn ConstructionScript)