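; Paint bucket actor that takes a paint brush through a dipping motion, then hands it back to the brush movement actor.
; DipBrush stores the brush and start position, and Tick lerps the brush's MoverPos to DipFrom.
; Each arrival triggers a one-tick lerp toward DipTo and increments a never-reset counter.
; At ten dips, it returns the brush to BP_PaintBrushMovement, changes that actor's state and clears its reference.
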(event EventBeginPlay)

(event Collision|EventActorBeginOverlap
  (params (OtherActor :type Actor%20Object%20Reference)))

(event EventTick
  (params (DeltaSeconds :type Float%20%28single-precision%29))
  (bind _dip_from (Variables|Default|GetDip_from))
  (bind _returnvalue (Transformation|GetWorldLocation _dip_from))
  (if (Variables|Default|GetIsAtDipFrom)
    (bind _output_get (Variables|Default|Setalpha (+ (Variables|Default|Getalpha) (* 3 DeltaSeconds))))
    (Variables|/Game/Blueprints/PaintBrush/BP_PaintBrush.BP_PaintBrush_C|SetMoverPos (Variables|Default|GetPaintBrush) (Math|Vector|Lerp(Vector) _returnvalue (Transformation|GetWorldLocation (Variables|Default|GetDip_to)) _output_get))
    (Variables|Default|SetDips (+ (Variables|Default|GetDips) 1))
    (if (== (Variables|Default|GetDips) 10)
      (bind _returnvalue_2 (Actor|GetActorOfClass "/Game/Blueprints/PaintBrush/BP_PaintBrushMovement.BP_PaintBrushMovement_C"))
      (Variables|/Game/Blueprints/PaintBrush/BP_PaintBrushMovement.BP_PaintBrushMovement_C|SetPaintBrush _returnvalue_2 (Variables|Default|GetPaintBrush))
      (Variables|Default|SetPaintBrush 0)
      (Variables|/Game/Blueprints/PaintBrush/BP_PaintBrushMovement.BP_PaintBrushMovement_C|SetState _returnvalue_2 "NewEnumerator3")
      (Variables|Default|SetIsAtDipFrom false)
      (Variables|Default|Setalpha 0.0)
      (else
        (Variables|Default|SetIsAtDipFrom false)
        (Variables|Default|Setalpha 0.0)
        (Variables|Default|SetMoverPos (Transformation|GetWorldLocation (Variables|/Game/Blueprints/PaintBrush/BP_PaintBrush.BP_PaintBrush_C|GetPaintBrushHandle (Variables|Default|GetPaintBrush))))))
    (else
      (Utilities|IsValid (Variables|Default|GetPaintBrush)
        (:Is%20Valid
          (bind _output_get_2 (Variables|Default|Setalpha (+ (Variables|Default|Getalpha) (* 3 DeltaSeconds))))
          (Variables|/Game/Blueprints/PaintBrush/BP_PaintBrush.BP_PaintBrush_C|SetMoverPos (Variables|Default|GetPaintBrush) (Math|Vector|Lerp(Vector) (Variables|Default|GetMoverPos) _returnvalue _output_get_2))
          (if (> _output_get_2 1.0)
            (Variables|/Game/Blueprints/PaintBrush/BP_PaintBrush.BP_PaintBrush_C|SetMoverPos (Variables|Default|GetPaintBrush) _returnvalue)
            (Variables|Default|SetIsAtDipFrom true)
            (Variables|Default|Setalpha 0.0)))))))

(fn ConstructionScript)

(fn DipBrush
  (params (paint%20brush :type BP%20Paint%20Brush%20Object%20Reference) (Position :type Vector))
  (if (not (== paint%20brush (Variables|Default|GetPaintBrush)))
    ;[1 1 1] Set Paintbrush Variable
    (Variables|Default|SetPaintBrush paint%20brush)
    (Variables|Default|SetMoverPos Position)))