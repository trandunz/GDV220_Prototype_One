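; BP_PaintBrush is a movable paint brush actor that leaves paint decals on the ground and plays a sound from BeginPlay.
; Each tick it moves its AnchorPoint to a position set through SetMoverPos and, while the handle is low, spawns BP_PaintDecal at ground level on a short timer.
; It also polls DayNightManager every tick, switching the handle between wood and fire materials and showing its point light only at night.
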(event EventBeginPlay
  (bind _audio (Variables|Default|GetAudio))
  (Audio|Components|Audio|SetSound _audio "/Game/Audio/MiniProd/Implemented/PaintBrush_Cue.PaintBrush_Cue")
  (Audio|Components|Audio|Play _audio 0.0)
  (bind _returnvalue (Actor|GetActorOfClass "/Game/DayNightCycle/DayNightManager.DayNightManager_C"))
  (Variables|Default|SetDayNightManager _returnvalue))

(event Collision|EventActorBeginOverlap
  (params (OtherActor :type Actor%20Object%20Reference)))

(event EventTick
  (params (DeltaSeconds :type Float%20%28single-precision%29))
  (bind _paintbrushhandle (Variables|Default|GetPaintBrushHandle))
  (Variables|Default|SetdecalTimer (+ DeltaSeconds (Variables|Default|GetdecalTimer)))
  (Utilities|FlowControl|Sequence
    (:then_0
      (Transformation|SetWorldLocation (Variables|Default|GetAnchorPoint) (Variables|Default|GetMoverPos) false false)
      (if (< (.Z (Math|Vector|BreakVector (Transformation|GetWorldLocation (Variables|Default|GetPaintBrushHandle)))) 5e+01)
        (if (> (Variables|Default|GetdecalTimer) 0.05)
          (Variables|Default|SetdecalTimer 0.0)
          (CallFunction|SpawnDecal))))
    (:then_1
      ;[1 1 1] Paint Brush Light
      (if (Variables|/Game/DayNightCycle/DayNightManager.DayNightManager_C|GetIsDay (Variables|Default|GetDayNightManager))
        (Rendering|Material|SetMaterial _paintbrushhandle 0 "/Game/StarterContent/Materials/M_Wood_Pine.M_Wood_Pine")
        (Rendering|SetVisibility (Variables|Default|GetPointLight) false false)
        (else
          (Rendering|Material|SetMaterial _paintbrushhandle 0 "/Game/EnvironmentMeshes/EnvironmentMaterials/MI_Fire.MI_Fire")
          (Rendering|SetVisibility (Variables|Default|GetPointLight) true false))))))

(fn ConstructionScript)

(fn SetMoverPos
  (params (position :type Vector))
  (Variables|Default|SetMoverPos position))

(fn SpawnDecal
  (bind _paintbrushhandle (Variables|Default|GetPaintBrushHandle))
  (bind _returnvalue (Transformation|GetWorldLocation _paintbrushhandle))
  (bind (_x _y) (Math|Vector|BreakVector _returnvalue))
  (Game|SpawnActorfromClass "/Game/Blueprints/PaintBrush/BP_PaintDecal.BP_PaintDecal_C" (Math|Transform|MakeTransform (Math|Vector|MakeVector _x _y 0.0) "0, 0, 0" "1,1,1") "Undefined" 0 0))