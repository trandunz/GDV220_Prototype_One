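; Drives BP_PaintBrush through a Tick state machine, moving a Mover and copying its position to the brush.
; The brush orbits with sine bobbing, handing off to any nearby bucket for dipping, and lerps to a wait bucket while InTower.
; At night, AI perception of a sleeping card soldier triggers an attack, then a gloating orbit with slap sounds over the victim.
; It returns toward the player afterward or when too far away.
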(event OnTargetPerceptionUpdated(AIPerception)
  (params (Actor :type Actor%20Object%20Reference) (Stimulus :type AI%20Stimulus%20Structure))
  (switch Utilities|FlowControl|Switch|SwitchonEnum_PaintBrushStsate (Variables|Default|GetState)
    (:NewEnumerator0
      (CallFunction|CheckPerception Actor Stimulus))
    (:NewEnumerator4
      (Variables|Default|SetSoldierSpottedWhileGloating true))))

(event EventBeginPlay
  ;[1 1 1] Set Paintbrush Variable
  (bind _returnvalue (Actor|GetActorOfClass "/Game/Blueprints/PaintBrush/BP_PaintBrush.BP_PaintBrush_C"))
  (Variables|Default|SetPaintBrush _returnvalue)
  (Variables|Default|SetState "NewEnumerator0")
  (bind _outactors (Actor|GetAllActorsOfClass "/Game/Blueprints/PaintBrush/BP_Bucket.BP_Bucket_C"))
  (Variables|Default|SetBuckets _outactors))

(event EventTick
  (params (DeltaSeconds :type Float%20%28single-precision%29))
  (bind _paintbrush (Variables|Default|GetPaintBrush))
  (bind _asplayer_prefs (Utilities|Casting|CastToPlayerPrefs (Game|GetGameInstance)))
  (if (Variables|/Game/Prefabs/PlayerPrefs.PlayerPrefs_C|GetInTower _asplayer_prefs)
    (bind _returnvalue (Actor|GetActorOfClass "/Game/Blueprints/PaintBrush/BP_WaitBucket.BP_WaitBucket_C"))
    (Utilities|IsValid _paintbrush
      (:Is%20Valid
        (Variables|/Game/Blueprints/PaintBrush/BP_PaintBrush.BP_PaintBrush_C|SetMoverPos _paintbrush (Math|Vector|Lerp(Vector) (Variables|/Game/Blueprints/PaintBrush/BP_PaintBrush.BP_PaintBrush_C|GetMoverPos (Variables|Default|GetPaintBrush)) (Transformation|GetWorldLocation (Variables|/Game/Blueprints/PaintBrush/BP_WaitBucket.BP_WaitBucket_C|GetWaitPos _returnvalue)) DeltaSeconds))
        (Variables|Default|SetState "NewEnumerator3")
        (Variables|Default|SetCacheCurrentLocation (Variables|/Game/Blueprints/PaintBrush/BP_PaintBrush.BP_PaintBrush_C|GetMoverPos (Variables|Default|GetPaintBrush)))))
    (else
      (Variables|Default|SetDeltaSeconds DeltaSeconds)
      (switch Utilities|FlowControl|Switch|SwitchonEnum_PaintBrushStsate (Variables|Default|GetState)
        (:NewEnumerator0
          (CallFunction|Orbit DeltaSeconds (Transformation|GetWorldLocation (Variables|Default|GetCollisionComponent)))
          (bind _returnvalue_2 (Actor|GetActorOfClass "/Game/DayNightCycle/DayNightManager.DayNightManager_C"))
          (Variables|Default|SetDayNightManager _returnvalue_2))
        (:NewEnumerator1
          (CallFunction|AttackSoldier DeltaSeconds))
        (:NewEnumerator2
          (CallFunction|DipBrush DeltaSeconds))
        (:NewEnumerator3
          (CallFunction|BacktoOrbit))
        (:NewEnumerator4
          (CallFunction|Gloat (Transformation|GetWorldLocation (Variables|/Game/NPC/Card_Soldier/Card_Soldier/NPC_Card_Soldier.NPC_Card_Soldier_C|GetPaintBrushTarget (Variables|Default|GetSoldierToAttack)))))))))

(fn ConstructionScript)

(fn Orbit
  (params (DeltaSeconds :type Float%20%28single-precision%29) (OrbitOrigin :type Vector))
  (bind (_x _y _z) (Math|Vector|BreakVector OrbitOrigin))
  (bind _radius (Variables|Default|Getradius))
  (CallFunction|CheckforBuckets)
  ;[1 1 1] Apply Speed, increment Counter
  (bind _output_get (Variables|Default|Setcounter (+ (Variables|Default|Getcounter) (* (Variables|Default|GetOrbitSpeed) DeltaSeconds))))
  ;[1 1 1] Set T of the Parametric Form equation
  (Variables|Default|Sett (+ (/ (* (Math|Trig|Sin(Radians) _output_get) (* (Math|Trig|GetPI) 2.0)) 2.0) (Math|Trig|GetPI)))
  (CallFunction|SetMoverPos (Math|Vector|MakeVector (+ _x (* (Math|Trig|Cos(Radians) (Variables|Default|Getcounter)) _radius)) (+ _y (* (Math|Trig|Sin(Radians) (Variables|Default|Getcounter)) _radius)) (+ _z (* (Math|Trig|Sin(Radians) (* (Variables|Default|GetUpDownSpeed) (Variables|Default|Getcounter))) (Variables|Default|GetUpDownDistance))))))

(fn AttackSoldier
  (params (Delta%20Seconds :type Float%20%28single-precision%29))
  (if (> (Math|Vector|Distance(Vector) (Transformation|GetWorldLocation (Variables|Default|GetMover)) (Transformation|GetWorldLocation (Variables|/Script/Engine.Character|GetCapsuleComponent (Game|GetPlayerCharacter 0)))) 1e+03)
    (Variables|Default|SetCacheCurrentLocation (Transformation|GetWorldLocation (Variables|Default|GetMover)))
    (Variables|Default|SetGloatTimer 0.0)
    (CallFunction|BacktoOrbit)
    (else
      ;[1 1 1] Check if Card Soldier has already been attacked
      (if (Variables|/Game/NPC/Card_Soldier/Card_Soldier/NPC_Card_Soldier.NPC_Card_Soldier_C|GetIsPlatformMode (Variables|Default|GetSoldierToAttack))
        (Variables|Default|SetIsGloating true)
        (Variables|Default|SetState "NewEnumerator4")
        (else
          ;[1 1 1] Check if Paint Brush is at the card soldier
          (bind _targettohit (Default|GetPaintBrushTarget (Variables|Default|GetSoldierToAttack)))
          (if (< (Math|Vector|Distance(Vector) (Transformation|GetWorldLocation (Variables|Default|GetMover)) _targettohit) 1e+01)
            ;[1 1 1] Attack
            (Default|GetHit (Variables|Default|GetSoldierToAttack))
            (Variables|Default|SetLerpAlpha 0.0)
            (Audio|PlaySoundatLocation "/Game/Audio/MiniProd/Slaps/gloating_Cue.gloating_Cue" _targettohit "0, 0, 0" 1.0 1.0 0.0 "/Game/Audio/PaintBrush_Attenuation.PaintBrush_Attenuation" 0 0)
            (else
              ;[1 1 1] Lerp between current location and soldier location
              (bind _targettohit_2 (Default|GetPaintBrushTarget (Variables|Default|GetSoldierToAttack)))
              (bind _output_get (Variables|Default|SetLerpAlpha (+ Delta%20Seconds (Variables|Default|GetLerpAlpha))))
              (CallFunction|Lerpto (Variables|Default|GetCacheCurrentLocation) _targettohit_2 _output_get 1.5))))))))

(fn CheckPerception
  (params (Actor :type Actor%20Object%20Reference) (AIStimulus :type AI%20Stimulus%20Structure))
  (if (not (Variables|/Game/DayNightCycle/DayNightManager.DayNightManager_C|GetIsDay (Variables|Default|GetDayNightManager)))
    (bind _asnpc_card_soldier (Utilities|Casting|CastToNPC_Card_Soldier Actor))
    ;[1 1 1] Check if soldier is not already set, is not attacked, is sleeping, and successfully sensed
    (if (not (== _asnpc_card_soldier (Variables|Default|GetSoldierToAttack)))
      (if (not (Variables|/Game/NPC/Card_Soldier/Card_Soldier/NPC_Card_Soldier.NPC_Card_Soldier_C|GetIsPlatformMode _asnpc_card_soldier))
        (if (Variables|/Game/NPC/Card_Soldier/Card_Soldier/NPC_Card_Soldier.NPC_Card_Soldier_C|GetIsSleeping _asnpc_card_soldier)
          (if (.bSuccessfullySensed (Utilities|Struct|BreakAIStimulus AIStimulus))
            (Variables|Default|SetState "NewEnumerator1")
            (Variables|Default|SetSoldierToAttack _asnpc_card_soldier)
            (Variables|Default|SetCacheCurrentLocation (Transformation|GetWorldLocation (Variables|Default|GetMover)))))))))

(fn Gloat
  (params (DeadSoldierLocation :type Vector))
  (bind (_x _y) (Math|Vector|BreakVector DeadSoldierLocation))
  (bind _gloatspeed (Variables|Default|GetGloatSpeed))
  (if (Variables|Default|GetIsGloating)
    (CallFunction|Orbit _gloatspeed (Math|Vector|MakeVector _x _y 3e+01))
    (Variables|Default|SetGloatTimer (+ _gloatspeed (Variables|Default|GetGloatTimer)))
    (Utilities|FlowControl|Sequence
      (:then_0
        (CallFunction|PlaySlapSound))
      (:then_1
        (if (> (Variables|Default|GetGloatTimer) 5.0)
          (Variables|Default|SetIsGloating false))))
    (else
      (Variables|Default|SetCacheCurrentLocation (Transformation|GetWorldLocation (Variables|Default|GetMover)))
      (Variables|Default|SetGloatTimer 0.0)
      (CallFunction|BacktoOrbit))))

(fn SetMoverPos
  (params (position :type Vector))
  ;[1 1 1] Set Mover position and PaintBrush varianble "MoverPos"
  (Transformation|SetWorldLocation (Variables|Default|GetMover) position false false)
  (Variables|/Game/Blueprints/PaintBrush/BP_PaintBrush.BP_PaintBrush_C|SetMoverPos (Variables|Default|GetPaintBrush) position))

(fn BacktoOrbit
  (bind _returnvalue (Game|GetPlayerCharacter 0))
  (bind _paintbrush (Variables|Default|GetPaintBrush))
  (bind _returnvalue_2 (Transformation|GetActorLocation _returnvalue))
  (bind _moverpos (Variables|/Game/Blueprints/PaintBrush/BP_PaintBrush.BP_PaintBrush_C|GetMoverPos _paintbrush))
  (bind _output_get (Variables|Default|SetLerpAlpha (+ (Variables|Default|GetLerpAlpha) (Variables|Default|GetDeltaSeconds))))
  (if (< (Math|Vector|VectorLength (- _moverpos _returnvalue_2)) 5e+01)
    (Variables|Default|SetLerpAlpha 0.0)
    (Variables|Default|SetState "NewEnumerator0")
    (CallFunction|SetMoverPos _returnvalue_2)
    (else
      (CallFunction|Lerpto _moverpos _returnvalue_2 _output_get 0.1))))

(fn Lerpto
  (params (a :type Vector) (b :type Vector) (alpha :type Float%20%28single-precision%29) (speed :type Float%20%28single-precision%29))
  (CallFunction|SetMoverPos (Math|Vector|Lerp(Vector) a b (* alpha speed))))

(fn CheckforBuckets
  (for (_array_element _array_index) (Variables|Default|GetBuckets)
    (if (<= (Math|Vector|VectorLength (- (Transformation|GetWorldLocation (Variables|Default|GetMover)) (Transformation|GetActorLocation _array_element))) 3e+02)
      (Variables|Default|SetState "NewEnumerator2")
      (Variables|Default|SetDipBucketIndex _array_index)
      (Variables|Default|SetDipBrushLocation (Transformation|GetSocketLocation (Variables|/Game/Blueprints/PaintBrush/BP_Bucket.BP_Bucket_C|GetDip_from _array_element) "None"))
      (Variables|Default|SetLerpAlpha 0.0))))

(fn DipBrush
  (params (delta_seconds :type Float%20%28single-precision%29))
  (if (Variables|Default|GetisDipping)
    (Variables|Default|SetPaintBrush 0)
    (else
      (for (_array_element _array_index) (Variables|Default|GetBuckets)
        (if (== _array_index (Variables|Default|GetDipBucketIndex))
          (Default|DipBrush _array_element (Variables|Default|GetPaintBrush) (Transformation|GetWorldLocation (Variables|Default|GetMover)))
          (Variables|Default|SetisDipping true)
          (Utilities|Array|RemoveIndex (Variables|Default|GetBuckets) (Variables|Default|GetDipBucketIndex)))))))

(fn PlaySlapSound
  (bind _paintbrush (Variables|Default|GetPaintBrush))
  (bind _paintbrushhandle (Variables|/Game/Blueprints/PaintBrush/BP_PaintBrush.BP_PaintBrush_C|GetPaintBrushHandle _paintbrush))
  (bind _returnvalue (Transformation|GetWorldLocation _paintbrushhandle))
  (Variables|Default|Setslap%20delay (+ (Variables|Default|Getslap%20delay) (Utilities|Time|GetWorldDeltaSeconds)))
  (if (> (Variables|Default|Getslap%20delay) 0.3)
    (Variables|Default|Setslap%20delay 0.0)
    (if (< (.Z (Math|Vector|BreakVector _returnvalue)) 5e+01)
      (Audio|PlaySoundatLocation (.OutItem (Utilities|Array|Random (Variables|Default|GetSlapSounds))) _returnvalue "0, 0, 0" 1.0 1.0 0.0 0 0 0))))