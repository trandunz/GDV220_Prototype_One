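; BP_WaitBucket is a proximity marker actor that flags whether the player's paint brush is near it, recorded as being "in tower".
; On BeginPlay it caches the PlayerPrefs game instance.
; Every Tick it looks up the ThirdPersonCharacter, measures the distance from its BPPaintBrushMovement component to the bucket's root, and sets InTower true within a fixed radius, false otherwise.
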(event EventBeginPlay
  (bind _asplayer_prefs (Utilities|Casting|CastToPlayerPrefs (Game|GetGameInstance)))
  (Variables|Default|SetAs%20Player%20Prefs _asplayer_prefs))

(event Collision|EventActorBeginOverlap
  (params (OtherActor :type Actor%20Object%20Reference)))

(event EventTick
  (params (DeltaSeconds :type Float%20%28single-precision%29))
  (bind _as_player_prefs (Variables|Default|GetAs%20Player%20Prefs))
  (bind _returnvalue (Actor|GetActorOfClass "/Game/ThirdPersonBP/Blueprints/ThirdPersonCharacter.ThirdPersonCharacter_C"))
  (if (< (Math|Vector|VectorLength (- (Transformation|GetWorldLocation (Variables|/Game/ThirdPersonBP/Blueprints/ThirdPersonCharacter.ThirdPersonCharacter_C|GetBP_PaintBrushMovement _returnvalue)) (Transformation|GetWorldLocation (Variables|Default|GetDefaultSceneRoot)))) 5e+02)
    (Variables|/Game/Prefabs/PlayerPrefs.PlayerPrefs_C|SetInTower _as_player_prefs true)
    (else
      (Variables|/Game/Prefabs/PlayerPrefs.PlayerPrefs_C|SetInTower _as_player_prefs false))))

(fn ConstructionScript)