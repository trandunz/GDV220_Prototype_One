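; SignMap is a map sign that opens a map view when its trigger is overlapped.
; BeginPlay hides Paper2D sprites on mushroom and card soldier NPCs, checkpoints and end-game triggers, and overlap reveals them as apparent map markers.
; Overlap also plays a sound, moves MapCam-tagged actors to the player's XY, blocks move input and zooms the stopped character's fixed camera onto the map.
; It sets IsPlayerInMap but contains no exit logic.
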(event OnComponentBeginOverlap(Trigger)
  (params (OverlappedComponent :type Primitive%20Component%20Object%20Reference) (OtherActor :type Actor%20Object%20Reference) (OtherComp :type Primitive%20Component%20Object%20Reference) (OtherBodyIndex :type Integer) (bFromSweep :type Boolean) (SweepResult :type Hit%20Result%20Structure%20%28by%20ref%29))
  (bind _returnvalue (Game|GetPlayerCharacter 0))
  (bind _returnvalue_2 (Transformation|GetActorLocation _returnvalue))
  (bind (_x _y) (Math|Vector|BreakVector _returnvalue_2))
  (Audio|PlaySound2D "/Game/Audio/Sfx/sfx_map_Cue.sfx_map_Cue" 1.0 1.0 0.0 0 0)
  (bind _outactors (Actor|GetAllActorswithTag "MapCam"))
  (for _array_element _outactors
    (Transformation|SetActorLocation _array_element (Math|Vector|MakeVector _x _y (.Z (Math|Vector|BreakVector (Transformation|GetActorLocation _array_element)))) false true))
  (Variables|Default|SetIsPlayerInMap true)
  (bind _asthird_person_character (Utilities|Casting|CastToThirdPersonCharacter OtherActor))
  (Input|SetIgnoreMoveInput (Game|GetPlayerController 0) true)
  (Default|ZoominonObject _asthird_person_character (Transformation|GetWorldLocation (Variables|Default|GetMap1)) (Transformation|GetWorldLocation (Variables|Default|GetViewLocation)))
  (Variables|/Game/ThirdPersonBP/Blueprints/ThirdPersonCharacter.ThirdPersonCharacter_C|SetCameraIsFixed _asthird_person_character true)
  (Variables|/Script/Engine.MovementComponent|SetVelocity (Variables|/Script/Engine.Character|GetCharacterMovement _asthird_person_character) "0, 0, 0")
  (Utilities|FlowControl|Sequence
    (:then_0
      (bind _outactors_2 (Actor|GetAllActorsOfClass "/Game/NPC/Mushroom/NPC_Mushroom.NPC_Mushroom_C"))
      (for _array_element_2 _outactors_2
        (Rendering|SetVisibility (Actor|GetComponentbyClass _array_element_2 "/Script/Paper2D.PaperSpriteComponent") true false)))
    (:then_1
      (bind _outactors_3 (Actor|GetAllActorsOfClass "/Game/NPC/Card_Soldier/Card_Soldier/NPC_Card_Soldier.NPC_Card_Soldier_C"))
      (for _array_element_3 _outactors_3
        (Rendering|SetVisibility (Actor|GetComponentbyClass _array_element_3 "/Script/Paper2D.PaperSpriteComponent") true false)))
    (:then_2
      (bind _outactors_4 (Actor|GetAllActorsOfClass "/Game/Blueprints/Checkpoint.Checkpoint_C"))
      (for _array_element_4 _outactors_4
        (Rendering|SetVisibility (Actor|GetComponentbyClass _array_element_4 "/Script/Paper2D.PaperSpriteComponent") true false)))
    (:then_3
      (bind _outactors_5 (Actor|GetAllActorsOfClass "/Game/Blueprints/EndGameTrigger.EndGameTrigger_C"))
      (for _array_element_5 _outactors_5
        (Rendering|SetVisibility (Actor|GetComponentbyClass _array_element_5 "/Script/Paper2D.PaperSpriteComponent") true false)))))

(event EventBeginPlay
  (Utilities|FlowControl|Sequence
    (:then_0
      (bind _outactors (Actor|GetAllActorsOfClass "/Game/NPC/Mushroom/NPC_Mushroom.NPC_Mushroom_C"))
      (for _array_element _outactors
        (Rendering|SetVisibility (Actor|GetComponentbyClass _array_element "/Script/Paper2D.PaperSpriteComponent") false false)))
    (:then_1
      (bind _outactors_2 (Actor|GetAllActorsOfClass "/Game/NPC/Card_Soldier/Card_Soldier/NPC_Card_Soldier.NPC_Card_Soldier_C"))
      (for _array_element_2 _outactors_2
        (Rendering|SetVisibility (Actor|GetComponentbyClass _array_element_2 "/Script/Paper2D.PaperSpriteComponent") false false)))
    (:then_2
      (bind _outactors_3 (Actor|GetAllActorsOfClass "/Game/Blueprints/Checkpoint.Checkpoint_C"))
      (for _array_element_3 _outactors_3
        (Rendering|SetVisibility (Actor|GetComponentbyClass _array_element_3 "/Script/Paper2D.PaperSpriteComponent") false false)))
    (:then_3
      (bind _outactors_4 (Actor|GetAllActorsOfClass "/Game/Blueprints/EndGameTrigger.EndGameTrigger_C"))
      (for _array_element_4 _outactors_4
        (Rendering|SetVisibility (Actor|GetComponentbyClass _array_element_4 "/Script/Paper2D.PaperSpriteComponent") false false)))))

(fn ConstructionScript)