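; Blue small mushroom actor that swaps its toadstool material between day and night versions.
; On BeginPlay it finds and caches the level's DayNightManager.
; Tick runs through a one-second Delay, so it polls the manager's IsDay flag about once a second and sets the mesh's first material slot to match.
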(event EventBeginPlay
  (bind _returnvalue (Actor|GetActorOfClass "/Game/DayNightCycle/DayNightManager.DayNightManager_C"))
  (Variables|Default|SetDayNightManager _returnvalue))

(event Collision|EventActorBeginOverlap
  (params (OtherActor :type Actor%20Object%20Reference)))

(event EventTick
  (params (DeltaSeconds :type Float%20%28single-precision%29))
  (Utilities|FlowControl|Delay 1.0)
  (if (Variables|/Game/DayNightCycle/DayNightManager.DayNightManager_C|GetIsDay (Variables|Default|GetDayNightManager))
    (Rendering|Material|SetMaterial (Variables|Default|GetSmallMushroom) 0 "/Game/EnvironmentMeshes/EnvironmentMaterials/MI_Toadstool_Day_2.MI_Toadstool_Day_2")
    (else
      (Rendering|Material|SetMaterial (Variables|Default|GetSmallMushroom) 0 "/Game/EnvironmentMeshes/EnvironmentMaterials/MI_Toadstool_Night_2.MI_Toadstool_Night_2"))))

(fn ConstructionScript)