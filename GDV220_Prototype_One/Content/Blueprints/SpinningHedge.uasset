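; Hedge actor that turns between a day yaw and a night yaw to follow the game's day/night state.
; Each Tick stores DeltaSeconds and calls Rotate, which looks up the DayNightManager by class and reads its IsDay flag.
; Rotate steps yaw toward the matching target at RotateSpeed, clamping on overshoot, with a plain numeric comparison and no angle wrapping.
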(event EventBeginPlay)

(event Collision|EventActorBeginOverlap
  (params (OtherActor :type Actor%20Object%20Reference)))

(event EventTick
  (params (DeltaSeconds :type Float%20%28single-precision%29))
  (Variables|Default|SetDelta%20Seconds DeltaSeconds)
  (CallFunction|Rotate))

(fn ConstructionScript)

(fn Rotate
  (bind _returnvalue (Transformation|GetActorRotation))
  (bind _returnvalue_2 (Transformation|GetActorRotation))
  (bind _returnvalue_3 (Transformation|GetActorRotation))
  (bind _returnvalue_4 (Transformation|GetActorRotation))
  (bind _returnvalue_5 (Transformation|GetActorRotation))
  (bind _returnvalue_6 (Transformation|GetActorRotation))
  (bind _returnvalue_7 (Transformation|GetActorRotation))
  (bind _returnvalue_8 (Transformation|GetActorRotation))
  (bind _dayrotationz (Variables|Default|GetDayRotationZ))
  (bind _dayrotationz_2 (Variables|Default|GetDayRotationZ))
  (bind _nightrotationz (Variables|Default|GetNightRotationZ))
  (bind _nightrotationz_2 (Variables|Default|GetNightRotationZ))
  (bind (_roll _pitch _yaw) (Math|Rotator|BreakRotator _returnvalue))
  (bind (_roll_2 _pitch_2 _yaw_2) (Math|Rotator|BreakRotator _returnvalue_2))
  (bind (_roll_3 _pitch_3 _yaw_3) (Math|Rotator|BreakRotator _returnvalue_3))
  (bind (_roll_4 _pitch_4 _yaw_4) (Math|Rotator|BreakRotator _returnvalue_4))
  (bind (_roll_5 _pitch_5 _yaw_5) (Math|Rotator|BreakRotator _returnvalue_5))
  (bind (_roll_6 _pitch_6 _yaw_6) (Math|Rotator|BreakRotator _returnvalue_6))
  (bind (_roll_7 _pitch_7 _yaw_7) (Math|Rotator|BreakRotator _returnvalue_7))
  (bind (_roll_8 _pitch_8 _yaw_8) (Math|Rotator|BreakRotator _returnvalue_8))
  (bind _returnvalue_9 (Actor|GetActorOfClass "/Game/DayNightCycle/DayNightManager.DayNightManager_C"))
  (if (Variables|/Game/DayNightCycle/DayNightManager.DayNightManager_C|GetIsDay _returnvalue_9)
    (Math|Float|CompareFloat (.Yaw (Math|Rotator|BreakRotator (Transformation|GetActorRotation))) (Variables|Default|GetDayRotationZ)
      (:>
        (Transformation|SetActorRotation (Math|Rotator|MakeRotator _roll_5 _pitch_5 (- _yaw_5 (* (Variables|Default|GetrotateSpeed) (Variables|Default|GetDelta%20Seconds)))))
        (if (< _yaw_4 _dayrotationz)
          (Transformation|SetActorRotation (Math|Rotator|MakeRotator _roll_4 _pitch_4 _dayrotationz))))
      (:<
        (Transformation|SetActorRotation (Math|Rotator|MakeRotator _roll_6 _pitch_6 (+ _yaw_6 (* (Variables|Default|GetrotateSpeed) (Variables|Default|GetDelta%20Seconds)))))
        (if (> _yaw_7 _dayrotationz_2)
          (Transformation|SetActorRotation (Math|Rotator|MakeRotator _roll_7 _pitch_7 _dayrotationz_2)))))
    (else
      (Math|Float|CompareFloat (.Yaw (Math|Rotator|BreakRotator (Transformation|GetActorRotation))) (Variables|Default|GetNightRotationZ)
        (:>
          (Transformation|SetActorRotation (Math|Rotator|MakeRotator _roll_2 _pitch_2 (- _yaw_2 (* (Variables|Default|GetrotateSpeed) (Variables|Default|GetDelta%20Seconds)))))
          (if (< _yaw_3 _nightrotationz)
            (Transformation|SetActorRotation (Math|Rotator|MakeRotator _roll_3 _pitch_3 _nightrotationz))))
        (:<
          (Transformation|SetActorRotation (Math|Rotator|MakeRotator _roll _pitch (+ _yaw (* (Variables|Default|GetrotateSpeed) (Variables|Default|GetDelta%20Seconds)))))
          (if (> _yaw_8 _nightrotationz_2)
            (Transformation|SetActorRotation (Math|Rotator|MakeRotator _roll_8 _pitch_8 _nightrotationz_2))))))))