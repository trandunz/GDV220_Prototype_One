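; BP_StreetLight is a street lamp that switches itself on at night and off during the day.
; On BeginPlay it caches the DayNightManager, then Tick passes through a one-second Delay to poll IsDay about once per second.
; By day it sets the mesh's second material slot to glass and hides the point light; at night it applies a fire material and shows the light.
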(event EventBeginPlay
  (bind _returnvalue (Actor|GetActorOfClass "/Game/DayNightCycle/DayNightManager.DayNightManager_C"))
  (Variables|Default|SetDayNightManager _returnvalue))

(event Collision|EventActorBeginOverlap
  (params (OtherActor :type Actor%20Object%20Reference)))

(event EventTick
  (params (DeltaSeconds :type Float%20%28single-precision%29))
  (Utilities|FlowControl|Delay 1.0)
  (if (Variables|/Game/DayNightCycle/DayNightManager.DayNightManager_C|GetIsDay (Variables|Default|GetDayNightManager))
    (Rendering|Material|SetMaterial (Variables|Default|GetStaticMesh) 1 "/Game/StarterContent/Materials/M_Glass.M_Glass")
    (Rendering|SetVisibility (Variables|Default|GetPointLight) false false)
    (else
      (Rendering|Material|SetMaterial (Variables|Default|GetStaticMesh) 1 "/Game/EnvironmentMeshes/EnvironmentMaterials/MI_Fire.MI_Fire")
      (Rendering|SetVisibility (Variables|Default|GetPointLight) true false))))

(fn ConstructionScript)