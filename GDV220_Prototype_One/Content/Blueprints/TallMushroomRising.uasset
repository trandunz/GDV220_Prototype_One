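; Tall mushroom actor that rises out of the ground while its IsRising flag is set, stopping once its Z reaches zero.
; Each rising tick moves it along its up vector, makes the player character look at it and plays a tower camera shake at the player.
; A rumble sound plays once at the player's location, gated by the rumble audio's stopped state and a played flag.
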(event EventBeginPlay)

(event Collision|EventActorBeginOverlap
  (params (OtherActor :type Actor%20Object%20Reference)))

(event EventTick
  (params (DeltaSeconds :type Float%20%28single-precision%29))
  (if (Variables|Default|GetisRising)
    (Transformation|SetActorLocation (+ (Transformation|GetActorLocation) (* (* (Transformation|GetActorUpVector) (Variables|Default|GetfSpeed)) DeltaSeconds)) false false)
    (bind _asthird_person_character (Utilities|Casting|CastToThirdPersonCharacter (Game|GetPlayerCharacter 0)))
    (Default|PlayerLookatLargeMushroom _asthird_person_character)
    (Camera|PlayWorldCameraShake "/Game/Blueprints/TowerCameraShake.TowerCameraShake_C" (Transformation|GetActorLocation _asthird_person_character) 0.0 5e+02)
    (Utilities|FlowControl|Sequence
      (:then_0
        (switch Utilities|FlowControl|Switch|SwitchonEAudioComponentPlayState (Audio|Components|Audio|GetPlayState (Variables|Default|Gettower_rumble_Cue))
          (:Stopped
            (if (not (Variables|Default|GetaudioHasPlayed))
              (Variables|Default|SetaudioHasPlayed true)
              (Audio|PlaySoundatLocation "/Game/Audio/MiniProd/Implemented/tower_rumble_Cue.tower_rumble_Cue" (Transformation|GetActorLocation (Game|GetPlayerCharacter 0)) "0, 0, 0" 1.0 1.0 0.0 0 0 0)))))
      (:then_1
        (if (>= (.z (Transformation|GetActorLocation)) 0.0)
          (Variables|Default|SetisRising false))))))

(fn ConstructionScript)