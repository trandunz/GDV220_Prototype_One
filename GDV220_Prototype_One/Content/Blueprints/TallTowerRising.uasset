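; Tower actor that rises out of its starting position when triggered, with camera shake and a rumble sound.
; A one-shot Rise event sets a flag that makes Tick move the actor along its up vector until it reaches a maximum Z height.
; While rising, Tick also calls the player character's look-at-tower function, shakes the camera around the player and plays the rumble once at the player's location.
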(event Custom|Rise
  (Utilities|FlowControl|DoOnce false
    (:Completed
      (Variables|Default|SetisRising true))))

(event EventBeginPlay
  (Audio|Components|Audio|SetSound (Variables|Default|GetAudio) "/Game/Audio/MiniProd/tower_rumble_Cue.tower_rumble_Cue"))

(event Collision|EventActorBeginOverlap
  (params (OtherActor :type Actor%20Object%20Reference)))

(event EventTick
  (params (DeltaSeconds :type Float%20%28single-precision%29))
  (if (Variables|Default|GetisRising)
    (Transformation|SetActorLocation (+ (Transformation|GetActorLocation) (* (* (Transformation|GetActorUpVector) (Variables|Default|GetFSpeed)) DeltaSeconds)) false false)
    (bind _asthird_person_character (Utilities|Casting|CastToThirdPersonCharacter (Game|GetPlayerCharacter 0)))
    (Default|PlayerLookatTower _asthird_person_character)
    (Camera|PlayWorldCameraShake "/Game/Blueprints/TowerCameraShake.TowerCameraShake_C" (Transformation|GetActorLocation _asthird_person_character) 0.0 5e+02)
    (Utilities|FlowControl|Sequence
      (:then_0
        (switch Utilities|FlowControl|Switch|SwitchonEAudioComponentPlayState (Audio|Components|Audio|GetPlayState (Variables|Default|GetAudio))
          (:Stopped
            (if (not (Variables|Default|GetaudioHasPlayed))
              (Variables|Default|SetaudioHasPlayed true)
              (Audio|PlaySoundatLocation "/Game/Audio/MiniProd/tower_rumble_Cue.tower_rumble_Cue" (Transformation|GetActorLocation (Game|GetPlayerCharacter 0)) "0, 0, 0" 1.0 1.0 0.0 0 0 0)))))
      (:then_1
        (if (>= (.z (Transformation|GetActorLocation)) (Variables|Default|GetfMaxZHeight))
          (Variables|Default|SetisRising false))))))

(fn ConstructionScript)